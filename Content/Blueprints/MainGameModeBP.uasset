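; Game mode Blueprint that, as wired, only prints "Login" on PostLogin.
; ChoosePlayerStart and SpawnDefaultPawnFor overrides are empty, as are BeginPlay, Tick and the construction script.
; Disconnected nodes hold unfinished experiments: claiming untaken PlayerStarts by tag, spawning a default pawn, and switching the view to a CameraActor found by object name.
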(event EventBeginPlay)

(event EventTick
  (params (DeltaSeconds :type Float%20%28single-precision%29)))

(event EventPostLogin
  (params (NewPlayer :type Player%20Controller%20Object%20Reference))
  (Development|PrintString "Login"))

(fn ConstructionScript)

(fn ChoosePlayerStart
  (params (Player :type Controller%20Object%20Reference)))

(fn SpawnDefaultPawnfor
  (params (NewPlayer :type Controller%20Object%20Reference) (StartSpot :type Actor%20Object%20Reference)))