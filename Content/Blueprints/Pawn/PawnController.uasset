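; Player controller Blueprint holding an unfinished key-driven movement scheme for MainPawnPB, most of which is not wired up.
; Three AnyKey release events clear the Back, Left and Right pressed flags, regardless of which key was released.
; Disconnected logic would set flags by comparing key display names to direction variables, then drive the pawn's CustomMovement and CustomMoveRight for forward and right only.
; BeginPlay and Tick are empty, so nothing here moves the pawn.
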(event EventBeginPlay)

(event EventTick
  (params (DeltaSeconds :type Float%20%28single-precision%29)))

(event Input|KeyboardEvents|AnyKey
  (params (Key :type Key%20Structure))
  (:Released
    (Variables|Default|SetRightPressed false)))

(event Input|KeyboardEvents|AnyKey
  (params (Key :type Key%20Structure)))

(event Input|KeyboardEvents|AnyKey
  (params (Key :type Key%20Structure))
  (:Released
    (Variables|Default|SetBackPressed false)))

(event Input|KeyboardEvents|AnyKey
  (params (Key :type Key%20Structure))
  (:Released
    (Variables|Default|SetLeftPressed false)))

(fn ConstructionScript)