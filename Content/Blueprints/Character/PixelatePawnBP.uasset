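; PixelatePawnBP is a player-controlled pawn that drives a physics-simulated static mesh with forward and turn axis inputs.
; MoveForward adds linear velocity along the mesh's forward vector, scaled by input and delta time.
; MoveRight adds the raw axis value to the mesh's world yaw, zeroing pitch and roll, without delta-time scaling.
; The PlayerNumber text displays the current MoveForward axis value rather than a player number.
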(event EventBeginPlay)

(event Collision|EventActorBeginOverlap
  (params (OtherActor :type Actor%20Object%20Reference)))

(event EventTick
  (params (DeltaSeconds :type Float%20%28single-precision%29)))

(event Input|AxisEvents|InputAxisMoveForward
  (params (AxisValue :type Float%20%28single-precision%29))
  (CallFunction|MoveForward (* 1e+03 AxisValue))
  (Rendering|Components|TextRender|SetText (Variables|Default|GetPlayerNumber) (Utilities|Text|MakeLiteralText (Utilities|Text|ToText(Float) AxisValue "HalfToEven"))))

(event Input|AxisEvents|InputAxisMoveRight
  (params (AxisValue :type Float%20%28single-precision%29))
  (if (!= AxisValue 0.0)
    (CallFunction|RotatefromSelf AxisValue)))

(fn ConstructionScript)

(fn RotatefromSelf
  (params (Angle :type Float%20%28single-precision%29))
  (Transformation|SetWorldRotation (Variables|Default|GetStaticMesh) (Math|Rotator|MakeRotator 0.0 0.0 (+ (.Yaw (Math|Rotator|BreakRotator (Transformation|GetWorldRotation (Variables|Default|GetStaticMesh)))) (+ 0.0 Angle))) false false))

(fn MoveForward
  (params (Accel :type Float%20%28single-precision%29))
  (Physics|SetPhysicsLinearVelocity (Variables|Default|GetStaticMesh) (* (* (Math|Vector|GetForwardVector (Variables|Default|GetStaticMesh)) Accel) (* (Math|Float|MakeLiteralFloat 1.0) (Utilities|Time|GetWorldDeltaSeconds))) true "None"))